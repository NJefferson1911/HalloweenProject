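; BP_Thunder is a storm effect actor that fakes random lightning strikes with thunder sound.
; A looping timer started on BeginPlay rolls a weighted chance, then plays a 2D sound cue and turns the actor to a random yaw.
; The Flash graph briefly toggles a directional light's visibility, with nested weighted rolls adding up to two quick follow-up flashes for flicker.
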(event `self.ReceiveBeginPlay`
  (`KismetSystemLibrary.K2_SetTimerDelegate` (delegate `Chance for Thunder`) (`self.Min Seconds Between Lightning`) true))

(event `Chance for Thunder`
  (if (`KismetMathLibrary.RandomBoolWithWeight` (`self.Chance`))
    (`GameplayStatics.PlaySound2D` (`self.SoundCue`))
    (`self.K2_AddActorWorldRotation` (`KismetMathLibrary.MakeRotator` 0.0 0.0 (`KismetMathLibrary.RandomFloatInRange` 0.0 360.0)))
    (`self.Flash`)
    (if (`KismetMathLibrary.RandomBoolWithWeight` (`self.Chance for Second Flash`))
      (`KismetSystemLibrary.Delay` 0.05)
      (`self.Flash`)
      (if (`KismetMathLibrary.RandomBoolWithWeight` (`self.Chance for Second Flash`))
        (`KismetSystemLibrary.Delay` 0.03)
        (`self.Flash`)))))

(fn `UserConstructionScript`)